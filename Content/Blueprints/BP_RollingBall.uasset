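; BP_RollingBall is an actor Blueprint that spins itself around the vertical Z axis at a steady rate.
; Tick passes DegreesPerSec and delta time to RotateOnZ, which adds their product to the actor's yaw for frame-rate-independent rotation, keeping roll and pitch.
; BeginPlay calls Init, which is empty, and despite the name no logic moves or rolls the ball.
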(event EventBeginPlay
  (CallFunction|Init))

(event Collision|EventActorBeginOverlap
  (params (OtherActor :type Actor%20Object%20Reference)))

(event EventTick
  (params (DeltaSeconds :type Float%20%28single-precision%29))
  (CallFunction|RotateonZ (Variables|Default|GetDegreesPerSec) DeltaSeconds))

(fn ConstructionScript)

(fn RotateonZ
  (params (angle :type Float%20%28double-precision%29) (deltaTime :type Float%20%28double-precision%29))
  (bind _self self)
  (bind _returnvalue (Transformation|GetActorRotation _self))
  (Transformation|SetActorRotation _self (Math|Rotator|MakeRotator (.roll _returnvalue) (.pitch _returnvalue) (+ (.yaw _returnvalue) (* angle deltaTime))))
  (return))

(fn Init)