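; A VR push button that sinks when pressed and flags a RollingBall to change color.
; BeginPlay caches the resting position and a lowered position for the button.
; A sphere component entering the collision box lowers the button, plays an explosion sound and sets the ball's ChangeColor flag.
; Release is filtered differently: only a VRPawn actor ending overlap raises the button again.
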(event OnComponentBeginOverlap(CollisionBox)
  (params (OverlappedComponent :type Primitive%20Component%20Object%20Reference) (OtherActor :type Actor%20Object%20Reference) (OtherComp :type Primitive%20Component%20Object%20Reference) (OtherBodyIndex :type Integer) (bFromSweep :type Boolean) (SweepResult :type Hit%20Result%20Structure%20%28by%20ref%29))
  ;[1 1 1] Détection appui, enfonce le bouton
  (Utilities|Casting|CastToSphereComponent OtherComp)
  (Transformation|SetRelativeLocation (Variables|Default|GetButton) (Variables|Default|GetInPosition) false false)
  ;[1 1 1] Joue un son à l'appui
  (Audio|PlaySoundatLocation "/Game/StarterContent/Audio/Explosion02.Explosion02" (Transformation|GetActorLocation) "0, 0, 0" 1.0 1.0 0.0 0 0 0 0)
  ;[1 1 1] Appelle un changement de couleur
  (Variables|/Game/Blueprints/BP_RollingBall.BP_RollingBall_C|SetChangeColor (Variables|Default|GetRollingBall) true))

(event OnComponentEndOverlap(CollisionBox)
  (params (OverlappedComponent :type Primitive%20Component%20Object%20Reference) (OtherActor :type Actor%20Object%20Reference) (OtherComp :type Primitive%20Component%20Object%20Reference) (OtherBodyIndex :type Integer))
  ;[1 1 1] Détection relachement, remonte le bouton
  (Utilities|Casting|CastToVRPawn OtherActor)
  (Transformation|SetRelativeLocation (Variables|Default|GetButton) (Variables|Default|GetOutPosition) false false))

(event EventBeginPlay
  (bind _button (Variables|Default|GetButton))
  (bind _relativelocation (Variables|/Script/Engine.SceneComponent|GetRelativeLocation _button))
  ;[1 1 1] Initialisation
  (Variables|Default|SetOutPosition _relativelocation)
  (Variables|Default|SetInPosition (- _relativelocation "0.000000,0.000000,10.000000")))

(fn ConstructionScript)